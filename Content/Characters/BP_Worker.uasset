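; Worker character that gathers resources for its parent resource building, which it takes as Home on BeginPlay.
; A Tick-driven state machine finds the nearest resource within Home's range, walks to it and carries the harvest back.
; Timers end the harvesting and processing phases, after which Home receives the units and the search restarts.
; Movement uses direct per-tick world offsets without sweep, while animations and tool/resource visibility change between phases.
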(event `self.ReceiveBeginPlay`
  (bind _asbp_buiilding_resource (cast `/Game/Buildings/BP_Buiilding_Resource` (`self.GetParentActor`)))
  (set `self.Home` _asbp_buiilding_resource))

(event `self.ReceiveTick`
  (params (DeltaSeconds :type "Float (single-precision)"))
  (switch `/Game/Characters/E_WorkerState` (`self.State`)
    (:`NewEnumerator1`
      (`self.FindNearbyResource`))
    (:`NewEnumerator2`
      (`self.WalkToResource`))
    (:`NewEnumerator4`
      (`self.GoBackHome`))))

(fn `EndHarvesting`
  (bind _currenttargetresource (`self.CurrentTargetResource`))
  (set `self.State` "NewEnumerator4")
  (`SkeletalMeshComponent.PlayAnimation` (`self.SkeletalMeshComponent`) "/Game/Animations/A_Carrying.A_Carrying" true)
  (`SceneComponent.SetHiddenInGame` (`self.Tool`) true false)
  (`SceneComponent.SetHiddenInGame` (`self.Resource`) false false)
  (`/Engine/EditorBlueprintResources/StandardMacros.IsValid` _currenttargetresource
    (:`Is Valid`
      (bind _collectedamount (`/Game/Resources/BP_Resource.Harvest` _currenttargetresource (`self.MaxHarvestedUnits`)))
      (set `self.UnitsHarvested` _collectedamount))))

(fn `EndProcessing`
  (`self.StartLoop`)
  (`/Game/Buildings/BP_Buiilding_Resource.EndProcessing` (`self.Home`) (`self.UnitsHarvested`))
  (set `self.UnitsHarvested` 0))

(fn `FindNearbyResource`
  (bind (_distance _returnvalue) (`GameplayStatics.FindNearestActor` (`self.K2_GetActorLocation`) (`PrimitiveComponent.GetOverlappingActors` (`/Game/Buildings/BP_Buiilding_Resource.Range` (`self.Home`)) (`self.Resource Class`))))
  (`/Engine/EditorBlueprintResources/StandardMacros.IsValid` _returnvalue
    (:`Is Valid`
      (bind _asbp_resource (cast `/Game/Resources/BP_Resource` _returnvalue))
      (set `self.CurrentTargetResource` _asbp_resource)
      (set `self.State` "NewEnumerator2")
      (`SceneComponent.SetHiddenInGame` (`self.Tool`) false false)
      (`SceneComponent.SetHiddenInGame` (`self.Resource`) true false)
      (`SkeletalMeshComponent.PlayAnimation` (`self.SkeletalMeshComponent`) "/Game/Animations/A_Walking.A_Walking" true))))

(fn `GoBackHome`
  (bind _returnvalue (`self.K2_GetActorLocation`))
  (bind _returnvalue_2 (`self.K2_GetActorLocation` (`self.Home`)))
  (bind _returnvalue_3 (- _returnvalue_2 _returnvalue))
  (`/Engine/EditorBlueprintResources/StandardMacros.IsValid` (`self.Home`)
    (:`Is Valid`
      ;[1 1 1] Move Towards Target
      (`self.K2_AddActorWorldOffset` (* (`KismetMathLibrary.Normal` _returnvalue_3) (`self.CarrySpeed`)))
      ;[1 1 1] Rotate to look at target
      (`self.K2_SetActorRotation` (`KismetMathLibrary.FindLookAtRotation` _returnvalue _returnvalue_2))
      ;[1 1 1] Change state and animation
      (if (<= (`KismetMathLibrary.VSize` _returnvalue_3) 5.0)
        (`self.StartProcessing`)))))

(fn `StartHarvesting`
  (`KismetSystemLibrary.K2_SetTimer` null "EndHarvesting" 5.0)
  (set `self.State` "NewEnumerator3")
  (`SkeletalMeshComponent.PlayAnimation` (`self.SkeletalMeshComponent`) "/Game/Animations/A_Harvesting.A_Harvesting" true))

(fn `StartLoop`
  (set `self.State` "NewEnumerator1"))

(fn `StartProcessing`
  (set `self.State` "NewEnumerator5")
  (`KismetSystemLibrary.K2_SetTimer` null "EndProcessing" (`self.ProcessingDuration`))
  (`/Game/Buildings/BP_Buiilding_Resource.StartProcessing` (`self.Home`)))

(fn `UserConstructionScript`)

(fn `WalkToResource`
  (bind _returnvalue (`self.K2_GetActorLocation`))
  (bind _returnvalue_2 (`self.K2_GetActorLocation` (`self.CurrentTargetResource`)))
  (bind _returnvalue_3 (- _returnvalue_2 _returnvalue))
  (`/Engine/EditorBlueprintResources/StandardMacros.IsValid` (`self.CurrentTargetResource`)
    (:`Is Valid`
      ;[1 1 1] Move Towards Target
      (`self.K2_AddActorWorldOffset` (* (`KismetMathLibrary.Normal` _returnvalue_3) (`self.MovementSpeed`)))
      ;[1 1 1] Rotate to look at target
      (`self.K2_SetActorRotation` (`KismetMathLibrary.FindLookAtRotation` _returnvalue _returnvalue_2))
      ;[1 1 1] Change state and animation
      (if (<= (`KismetMathLibrary.VSize` _returnvalue_3) (`/Game/Resources/BP_Resource.HarvestingDistance` (`self.CurrentTargetResource`)))
        (`self.StartHarvesting`)))))