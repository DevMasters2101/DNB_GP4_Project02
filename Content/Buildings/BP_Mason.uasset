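; BP_Mason is a mason building, a child of a parent building class that supplies placement and processing states.
; It overrides the state coloring to show green or red placement feedback while floating and the normal material when ready, reusing the Forge materials.
; Starting and ending processing call the parent and switch the PSFire particle effect on and off, while DoProcessing is left empty.
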(fn `DoProcessing`)

(fn `EndProcessing`
  (params (CollectedAmount :type Integer))
  (`parent.EndProcessing` CollectedAmount)
  (`ActorComponent.Deactivate` (`self.PS_Fire`)))

(fn `SetColorByState`
  (bind _result (`self.CanBePlaced`))
  (`PrimitiveComponent.SetMaterial` (`self.Mason`) 0 (select `/Game/Buildings/E_Building_State` (`self.State`) :`NewEnumerator0` (select `bool` _result :`false` "/Game/Materials/M_Forge_Red.M_Forge_Red" :`true` "/Game/Materials/M_Forge_Green.M_Forge_Green" :!type "MaterialInterface Object Reference") :`NewEnumerator1` "/Game/Materials/M_Forge.M_Forge")))

(fn `StartProcessing`
  (`parent.StartProcessing`)
  (`ActorComponent.Activate` (`self.PS_Fire`) false))

(fn `UserConstructionScript`
  (`parent.UserConstructionScript`))