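; Building manager actor that previews, moves and places buildings with the mouse cursor.
; It spawns a preview at BeginPlay and respawns it when the WBP_Build_Menu widget reports a new class.
; Tick traces under the cursor and moves the preview through SnapToGrid, which rounds X/Y to GridSize but has an unconnected return node.
; IA_Build completion places the preview if CanBePlaced allows, then spawns another.
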(event `self.ReceiveBeginPlay`
  (`self.SpawnBuilding`)
  (bind _returnvalue (`|CreateWidget` "/Game/UI/WBP_Build_Menu.WBP_Build_Menu_C"))
  (`UserWidget.AddToPlayerScreen` _returnvalue 0)
  (add `/Game/UI/WBP_Build_Menu.BuildingSelected` _returnvalue (delegate `BuildingSelected`)))

(event `BuildingSelected`
  (params (NewBuildingClass :type "/Game/Buildings/BP_Building Class Reference"))
  (set `self.BuildingClass` NewBuildingClass)
  (`self.SpawnBuilding`))

(event `self.ReceiveTick`
  (params (DeltaSeconds :type "Float (single-precision)"))
  (bind (_hitresult _returnvalue) (`PlayerController.GetHitResultUnderCursorByChannel` (`GameplayStatics.GetPlayerController` 0) "TraceTypeQuery3" true))
  ;[1 1 1] Move Building With Cursor
  (if (and (`KismetSystemLibrary.IsValid` (`self.BuildingToBePlaced`)) _returnvalue)
    (bind _outlocation (`self.SnapToGrid` (`.Location` (`GameplayStatics.BreakHitResult` _hitresult))))
    (`self.K2_SetActorLocation` (`self.BuildingToBePlaced`) _outlocation false false)))

(event `EnhancedInput|/Game/Inputs/IA_Build`
  (params (ActionValue :type Boolean) (ElapsedSeconds :type "Float (double-precision)") (TriggeredSeconds :type "Float (double-precision)") (InputAction :type "InputAction Object Reference" :default "/Game/Inputs/IA_Build.IA_Build"))
  (bind _buildingtobeplaced (`self.BuildingToBePlaced`))
  ;[1 1 1] Build By Click
  (:`Completed`
    (`/Engine/EditorBlueprintResources/StandardMacros.IsValid` _buildingtobeplaced
      (:`Is Valid`
        (bind _result (`/Game/Buildings/BP_Building.CanBePlaced` _buildingtobeplaced))
        (if _result
          (`/Game/Buildings/BP_Building.PlaceBuilding` _buildingtobeplaced)
          (set `self.BuildingToBePlaced` null)
          (`self.SpawnBuilding`))))))

(fn `SnapFloat`
  (params (InFloat :type "Float (double-precision)"))
  (returns (OutFloat :type "Float (double-precision)"))
  (bind _gridsize (`self.GridSize`))
  (return (* (`KismetMathLibrary.Round` (/ InFloat _gridsize)) _gridsize)))

(fn `SnapToGrid`
  (params (InLocation :type "Vector Structure"))
  (returns (OutLocation :type "Vector Structure"))
  (bind _outfloat (`self.SnapFloat` InLocation_X))
  (bind _outfloat_2 (`self.SnapFloat` InLocation_Y)))

(fn `SpawnBuilding`
  (bind _buildingtobeplaced (`self.BuildingToBePlaced`))
  (`/Engine/EditorBlueprintResources/StandardMacros.IsValid` _buildingtobeplaced
    (:`Is Valid`
      (`self.K2_DestroyActor` _buildingtobeplaced))
    (:`Is Not Valid`
      _))
  (bind _returnvalue (`|SpawnActorFromClass` (`self.BuildingClass`) (`KismetMathLibrary.MakeTransform` (0.0 0.0 0.0)) "Undefined" "MultiplyWithRoot" null null))
  (set `self.BuildingToBePlaced` _returnvalue))

(fn `UserConstructionScript`)