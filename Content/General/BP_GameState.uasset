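; BP_GameState tracks the player's resource stockpile and shows it in a top bar.
; On BeginPlay it creates WBP_Top_Bar and seeds starting amounts of trees, rocks and coins.
; SetResourceAmount writes a map keyed by resource class and pushes each value to the bar.
; AddResourceAmount adds to an existing entry or creates a new one through the same setter, keeping map and UI in sync.
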(event `self.ReceiveBeginPlay`
  (bind _returnvalue (`|CreateWidget` "/Game/UI/WBP_Top_Bar.WBP_Top_Bar_C"))
  (`UserWidget.AddToViewport` _returnvalue 0)
  (set `self.ResourceBar` _returnvalue)
  (`self.SetResourceAmount` "/Game/Resources/BP_Tree.BP_Tree_C" 50)
  (`self.SetResourceAmount` "/Game/Resources/BP_Rock.BP_Rock_C" 30)
  (`self.SetResourceAmount` "/Game/Resources/BP_Coin.BP_Coin_C" 10))

(fn `AddResourceAmount`
  (params (resourceClass :type "/Game/Resources/BP_Resource Class Reference") (resourceAmount :type Integer))
  (bind (_value _returnvalue) (`BlueprintMapLibrary.Map_Find` (`self.ResourceMap`) resourceClass))
  (if _returnvalue
    (`self.SetResourceAmount` resourceClass (+ _value resourceAmount))
    (else
      (`self.SetResourceAmount` resourceClass resourceAmount))))

(fn `SetResourceAmount`
  (params (resourceClass :type "/Game/Resources/BP_Resource Class Reference") (resourceAmount :type Integer))
  (`BlueprintMapLibrary.Map_Add` (`self.ResourceMap`) resourceClass resourceAmount)
  (`/Game/UI/WBP_Top_Bar.SetResourceAmount` (`self.ResourceBar`) resourceClass resourceAmount))

(fn `UserConstructionScript`)